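; Legacy Blueprint that runs a nine-stage vision test using arrays of letter components.
; Each stage sets a random letter's material visibility and stores its tag as the answer in BP_UserState.
; TestProcess uses that state's correct/incorrect counts to pass, retry or fail, but stages 6–8 ignore its result.
; Repeat polls KeyBoard_UI by looping timer, but TestProcess never waits, so timer-driven results are lost.
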(event `self.ReceiveBeginPlay`
  (`self.Set Text Array`)
  (`KismetSystemLibrary.Delay` 1.0 :!label _label)
  (bind _test_end (`self.Test Session`))
  (if _test_end
    _))

(event `Start vision test`
  (goto _label))

(fn `Repeat`
  (returns (NewParam :type Boolean))
  (bind _askey_board_ui (cast `/Game/EyeTest/Widget/Keyboard/KeyBoard_UI` (`self.WB_Object`)))
  (if (`/Game/EyeTest/Widget/Keyboard/KeyBoard_UI.Is User Responsed?` _askey_board_ui)
    (`KismetSystemLibrary.K2_ClearAndInvalidateTimerHandle` (`self.Func_RepeatHandler`))
    (return true)
    (else
      (bind _returnvalue (`KismetSystemLibrary.K2_SetTimer` null "Repeat" 0.1 true))
      (set `self.Func_RepeatHandler` _returnvalue))))

(fn `Set Text Array`
  (set `self.Array_01` (`|MakeArray` (`self.1-1T`) (`self.1-2Z`) (`self.1-3C`) (`self.1-4O`)))
  (set `self.Array_02` (`|MakeArray` (`self.2-1L`) (`self.2-2D`) (`self.2-3P`) (`self.2-4O`) (`self.2-5F`)))
  (set `self.Array_03` (`|MakeArray` (`self.3-1P`) (`self.3-2T`) (`self.3-3O`) (`self.3-4C`) (`self.3-5E`) (`self.3-6T`)))
  (set `self.Array_04` (`|MakeArray` (`self.4-1Z`) (`self.4-2L`) (`self.4-3P`) (`self.4-4E`) (`self.4-5D`) (`self.4-6T`) (`self.4-7C`)))
  (set `self.Array_05` (`|MakeArray` (`self.5-1E`) (`self.5-2T`) (`self.5-3O`) (`self.5-4D`) (`self.5-5C`) (`self.5-6F`) (`self.5-7O`)))
  (set `self.Array_06` (`|MakeArray` (`self.6-1D`) (`self.6-2P`) (`self.6-3C`) (`self.6-4Z`) (`self.6-5L`) (`self.6-6F`) (`self.6-7T`)))
  (set `self.Array_07` (`|MakeArray` (`self.7-1C`) (`self.7-2F`) (`self.7-3D`) (`self.7-4T`) (`self.7-5E`) (`self.7-6O`) (`self.7-7P`)))
  (set `self.Array_08` (`|MakeArray` (`self.8-1L`) (`self.8-2D`) (`self.8-3C`) (`self.8-4Z`) (`self.8-5O`) (`self.8-6T`) (`self.8-7E`)))
  (set `self.Array_09` (`|MakeArray` (`self.9-1P`) (`self.9-2F`) (`self.9-3O`) (`self.9-4D`) (`self.9-5T`) (`self.9-6E`) (`self.9-7L`)))
  (`KismetSystemLibrary.PrintString` "Set Array Successfully" true true (struct :`R` 0.897158 :`G` 1.0 :`A` 1.0) 66666.0)
  (return))

(fn `Set Visibility`
  (params (`input array` :type "Array of StaticMeshComponent Object Reference"))
  (returns (`output array` :type "Array of StaticMeshComponent Object Reference"))
  (bind _output (`|GetArrayItem` `input array` (`self.Array Index`)))
  (bind _returnvalue (`KismetTextLibrary.Conv_NameToText` (`|GetArrayItem` (`ActorComponent.ComponentTags` _output))))
  (set `self.Array Index` (`KismetMathLibrary.RandomIntegerInRange` 0 (- (`KismetArrayLibrary.Array_Length` `input array`) 1)))
  (`MeshComponent.SetScalarParameterValueOnMaterials` _output "Text visibility" 0.0)
  (`KismetSystemLibrary.PrintString` "text_Set successfully" true true (struct :`R` 0.173925 :`G` 1.0 :`B` 0.142638 :`A` 1.0) 10000.0)
  (bind _asbp_user_state (cast `/Game/EyeTest/Basic_Moduls/BP_UserState` (`GameplayStatics.GetPlayerState` 0)))
  (bind _output_get (set `/Game/EyeTest/Basic_Moduls/BP_UserState.Answer text` _returnvalue _asbp_user_state))
  (`KismetSystemLibrary.PrintString` "Text Spawned" true true (struct :`G` 0.66 :`B` 1.0 :`A` 1.0) 11111.0)
  (`KismetSystemLibrary.PrintString` "Answer Text Load Successfully" true true (struct :`G` 0.66 :`B` 1.0 :`A` 1.0) 11111.0)
  (`KismetSystemLibrary.PrintText` _returnvalue true true (struct :`G` 1.0 :`B` 0.255395 :`A` 1.0) 111111.0)
  (return `input array`))

(fn `Test Process`
  (params (`input array` :type "Array of StaticMeshComponent Object Reference"))
  (returns (Done :type Boolean))
  (bind _newparam (`self.Repeat`))
  (if _newparam
    (bind _asbp_user_state (cast `/Game/EyeTest/Basic_Moduls/BP_UserState` (`GameplayStatics.GetPlayerState` 0)))
    (if (`/Game/EyeTest/Basic_Moduls/BP_UserState.IsAnswercoreect` _asbp_user_state)
      (bind _result (`/Engine/EditorBlueprintResources/StandardMacros.IncrementInt` (`/Game/EyeTest/Basic_Moduls/BP_UserState.Correct Count` _asbp_user_state))
        (:`  `
          (if (>= (* _result 2) (* (/ (- (`KismetArrayLibrary.Array_Length` `input array`) 1) 2) 2))
            (`KismetSystemLibrary.PrintString` "정답수 과반수 이상." true true (struct :`G` 1.0 :`B` 0.975676 :`A` 1.0) 3.0)
            (`KismetSystemLibrary.PrintString` "다음 단계로 넘어갑니다." true true (struct :`G` 1.0 :`B` 0.981755 :`A` 1.0) 3.0)
            (return true)
            (else
              (`self.Set Visibility` `input array`)
              (`KismetSystemLibrary.PrintString` "동일한 시력 단계를 반복합니다." true true (struct :`G` 0.66 :`B` 1.0 :`A` 1.0) 3.0)
              (`KismetSystemLibrary.PrintString` "입력값 정답" true true (struct :`G` 0.66 :`B` 1.0 :`A` 1.0) 3.0)))))
      (else
        (bind _result_2 (`/Engine/EditorBlueprintResources/StandardMacros.IncrementInt` (`/Game/EyeTest/Basic_Moduls/BP_UserState.Incorrect Count` (`self.PlayerState`)))
          (:`  `
            (if (>= _result_2 3)
              (`KismetSystemLibrary.PrintString` "오답수 과반수 이상." true true (struct :`R` 1.0 :`G` 0.02448 :`A` 1.0) 1111.0)
              (`KismetSystemLibrary.PrintString` "검사를 종료합니다." true true (struct :`R` 1.0 :`G` 0.02448 :`A` 1.0) 311111.0)
              (return false)
              (else
                (`KismetSystemLibrary.PrintString` "동일한 시력 단계를 반복합니다." true true (struct :`R` 1.0 :`G` 0.02448 :`A` 1.0) 11113.0)
                (`KismetSystemLibrary.PrintString` "입력값 오답" true true (struct :`R` 1.0 :`G` 0.026519 :`A` 1.0) 1113.0)
                (`self.Set Visibility` `input array`)))))))
    (else
      (`KismetSystemLibrary.PrintString` "Repeat_False" true true (struct :`R` 0.404484 :`G` 0.6625 :`A` 1.0) 1112.0))))

(fn `Test Session`
  (returns (`Test End` :type Boolean))
  (bind _output_array (`self.Set Visibility` (`self.Array_01`)))
  (bind _done (`self.Test Process` _output_array))
  (if _done
    (bind _result (`/Engine/EditorBlueprintResources/StandardMacros.IncrementInt` (`self.TestCount`))
      (:`  `
        (set `self.TestCount` _result)
        (`KismetSystemLibrary.PrintString` "1단계 통과")
        (bind _output_array_2 (`self.Set Visibility` (`self.Array_02`)))
        (bind _done_2 (`self.Test Process` _output_array_2))
        (if _done_2
          (bind _result_2 (`/Engine/EditorBlueprintResources/StandardMacros.IncrementInt` (`self.TestCount`))
            (:`  `
              (set `self.TestCount` _result_2)
              (`KismetSystemLibrary.PrintString` "2단계 통과")
              (bind _output_array_3 (`self.Set Visibility` (`self.Array_03`)))
              (bind _done_3 (`self.Test Process` _output_array_3))
              (if _done_3
                (bind _result_3 (`/Engine/EditorBlueprintResources/StandardMacros.IncrementInt` (`self.TestCount`))
                  (:`  `
                    (set `self.TestCount` _result_3)
                    (`KismetSystemLibrary.PrintString` "3단계 통과")
                    (bind _output_array_4 (`self.Set Visibility` (`self.Array_04`)))
                    (bind _done_4 (`self.Test Process` _output_array_4))
                    (if _done_4
                      (bind _result_4 (`/Engine/EditorBlueprintResources/StandardMacros.IncrementInt` (`self.TestCount`))
                        (:`  `
                          (set `self.TestCount` _result_4)
                          (`KismetSystemLibrary.PrintString` "4단계 통과")
                          (bind _output_array_5 (`self.Set Visibility` (`self.Array_05`)))
                          (bind _done_5 (`self.Test Process` _output_array_5))
                          (if _done_5
                            (bind _result_5 (`/Engine/EditorBlueprintResources/StandardMacros.IncrementInt` (`self.TestCount`))
                              (:`  `
                                (set `self.TestCount` _result_5)
                                (`KismetSystemLibrary.PrintString` "5단계 통과")
                                (bind _output_array_6 (`self.Set Visibility` (`self.Array_06`)))
                                (`self.Test Process` _output_array_6)
                                (if true
                                  (bind _result_6 (`/Engine/EditorBlueprintResources/StandardMacros.IncrementInt` (`self.TestCount`))
                                    (:`  `
                                      (set `self.TestCount` _result_6)
                                      (`KismetSystemLibrary.PrintString` "6단계 통과")
                                      (bind _output_array_7 (`self.Set Visibility` (`self.Array_07`)))
                                      (`self.Test Process` _output_array_7)
                                      (if true
                                        (bind _result_7 (`/Engine/EditorBlueprintResources/StandardMacros.IncrementInt` (`self.TestCount`))
                                          (:`  `
                                            (set `self.TestCount` _result_7)
                                            (`KismetSystemLibrary.PrintString` "7단계 통과")
                                            (bind _output_array_8 (`self.Set Visibility` (`self.Array_08`)))
                                            (`self.Test Process` _output_array_8)
                                            (if true
                                              (bind _result_8 (`/Engine/EditorBlueprintResources/StandardMacros.IncrementInt` (`self.TestCount`))
                                                (:`  `
                                                  (set `self.TestCount` _result_8)
                                                  (`KismetSystemLibrary.PrintString` "8단계 통과")
                                                  (bind _output_array_9 (`self.Set Visibility` (`self.Array_09`)))
                                                  (bind _done_6 (`self.Test Process` _output_array_9))
                                                  (if _done_6
                                                    (bind _result_9 (`/Engine/EditorBlueprintResources/StandardMacros.IncrementInt` (`self.TestCount`))
                                                      (:`  `
                                                        (set `self.TestCount` _result_9)
                                                        (`KismetSystemLibrary.PrintString` "9단계 검사완료")
                                                        (return true)))
                                                    (else
                                                      (return false)))))
                                              (else
                                                (return false)))))
                                        (else
                                          (return false)))))
                                  (else
                                    (return false)))))
                            (else
                              (return false)))))
                      (else
                        (return false)))))
                (else
                  (return false)))))
          (else
            (return false)))))
    (else
      (return false))))

(fn `UserConstructionScript`)